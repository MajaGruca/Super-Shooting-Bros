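; Player character for a Paper2D side-scroller, with double jump, auto-repeat shooting, collectible points and lives.
; The MoveRight axis event also drives the fall-out-of-map check and flipbook updates through a state-selection function.
; Holding Shoot loops a delay that spawns projectiles, and a DoN reset on landing gates the launch-based second jump.
; Death costs a life, then respawns the character or pauses into the end menu.
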(event `Death`
  ;[1 1 1] Death
  (set `self.is Dead` true)
  (`KismetSystemLibrary.Delay` 0.33)
  (bind _output_get (set `self.Lives` (- (`self.Lives`) 1)))
  (`/Engine/EditorBlueprintResources/StandardMacros.CompareInt` _output_get
    (:`>`
      (`self.K2_SetActorLocationAndRotation` (`self.RespawnPoint`) (struct :`Yaw` -90.0))
      (set `self.is Dead` false))
    (:`==`
      (bind _returnvalue (`|CreateWidget` "/Game/EndMenu.EndMenu_C" null (`self.Points`) (`self.Lives`) :!label _label))
      (`UserWidget.AddToViewport` _returnvalue 0)
      (`WidgetBlueprintLibrary.SetInputMode_UIOnlyEx` (`GameplayStatics.GetPlayerController` 0) null)
      (`GameplayStatics.SetGamePaused` true))
    (:`<`
      (goto _label))))

(event `InputAction|Shoot`
  (params (Key :type "Key Structure"))
  ;[1 1 1] Shooting
  (:`Pressed`
    (set `self.isShooting` true)
    (`KismetSystemLibrary.Delay` 0.71 :!label _label_2)
    (if (`self.isShooting`)
      (`self.Shoot`)
      (goto _label_2)))
  (:`Released`
    (set `self.isShooting` false)))

(event `OutOfMap`
  ;[1 1 1] Out Of Map
  (`/Engine/EditorBlueprintResources/StandardMacros.CompareFloat` (.z (`self.K2_GetActorLocation`))
    (:`==`
      _)
    (:`<`
      _))
  (`self.Death`))

(event `InputAxis|MoveRight`
  (params (AxisValue :type "Float (single-precision)"))
  ;[1 1 1] Movement
  (`self.AddMovementInput` (0.0 -1.0 0.0) AxisValue)
  (`self.OutOfMap`)
  (`self.UpdateAnimation`)
  (`/Engine/EditorBlueprintResources/StandardMacros.CompareFloat` AxisValue
    (:`>`
      (`Controller.SetControlRotation` (`self.GetController`) (`KismetMathLibrary.MakeRotator` 0.0 0.0 -90.0)))
    (:`<`
      (`Controller.SetControlRotation` (`self.GetController`) (`KismetMathLibrary.MakeRotator` 0.0 0.0 90.0)))))

(event `InputAction|Jump`
  (params (Key :type "Key Structure"))
  ;[1 1 1] Jump + Double Jump
  (:`Pressed`
    (bind _counter (`/Engine/EditorBlueprintResources/StandardMacros.Do N` 2 :!label _label_3)
      (:`Exit`
        (switch `int` _counter
          (:`1`
            (`self.Jump`))
          (:`2`
            (`self.LaunchCharacter` (0.0 0.0 400.0) false true)
            (set `self.is Double Jumping` true)))))))

(event `self.ReceiveBeginPlay`
  ;[1 1 1] ReplicateEvent
  (`ActorComponent.SetIsReplicated` (`self.Sprite`) false))

(event `self.OnLanded`
  (params (Hit :type "HitResult Structure (by ref)"))
  ;[1 1 1] Jump + Double Jump
  (set `self.is Double Jumping` false)
  (goto _label_3 :!via `Reset`))

(event `UpdateAnimation`
  (bind _z (.z (`self.GetVelocity`)))
  ;[1 1 1] AnimationChange
  (set `self.is Moving` (!= (.y (`self.GetVelocity`)) 0.0))
  (set `self.is Jumping` (> _z 0.0))
  (set `self.is Falling` (< _z 0.0))
  (bind _outputflipbook (`self.Animation State Machine` (`self.is Moving`) (`self.is Jumping`) (`self.is Falling`) (`self.is Double Jumping`) (`self.is Dead`) (`self.isShooting`)))
  (`PaperFlipbookComponent.SetFlipbook` (`self.Sprite`) _outputflipbook))

(event `self.CapsuleComponent.OnComponentBeginOverlap`
  (params (OverlappedComponent :type "PrimitiveComponent Object Reference") (OtherActor :type "Actor Object Reference") (OtherComp :type "PrimitiveComponent Object Reference") (OtherBodyIndex :type Integer) (bFromSweep :type Boolean) (SweepResult :type "HitResult Structure (by ref)"))
  ;[1 1 1] CollectPoints
  (if (`KismetMathLibrary.ClassIsChildOf` (`GameplayStatics.GetObjectClass` OtherActor) "/Game/Blueprints/Collectible.Collectible_C")
    (bind _ascollectible (cast `/Game/Blueprints/Collectible` OtherActor))
    (set `self.Points` (+ (`/Game/Blueprints/Collectible.Value` _ascollectible) (`self.Points`)))))

(fn `Animation State Machine`
  (params (isMoving :type Boolean) (isJumping :type Boolean) (isFalling :type Boolean) (isDoubleJumping :type Boolean) (isDead :type Boolean) (isShooting :type Boolean))
  (returns (OutputFlipbook :type "PaperFlipbook Object Reference"))
  (locals (AnimationState :type "/Game/Data/AnimationState Enum" :default "NewEnumerator0") (isFallingLocal :type Boolean) (isMovingLocal :type Boolean) (isJumpingLocal :type Boolean) (isDoubleJumpingLocal :type Boolean) (isDeadLocal :type Boolean) (isShootingLocal :type Boolean))
  (set `local.isMovingLocal` isMoving)
  (set `local.isJumpingLocal` isJumping)
  (set `local.isFallingLocal` isFalling)
  (set `local.isDoubleJumpingLocal` isDoubleJumping)
  (set `local.isDeadLocal` isDead)
  (set `local.isShootingLocal` isShooting)
  (if (`NavMovementComponent.IsFalling` (`self.CharacterMovement`))
    (if (`local.isJumpingLocal`)
      (if (`local.isDoubleJumpingLocal`)
        (set `local.AnimationState` "NewEnumerator4")
        (else
          (set `local.AnimationState` "NewEnumerator2")))
      (else
        (set `local.AnimationState` "NewEnumerator3")))
    (elif (`local.isMovingLocal`)
      (set `local.AnimationState` "NewEnumerator1")
      (else
        (set `local.AnimationState` "NewEnumerator0"))))
  (if (`local.isShootingLocal`)
    (set `local.AnimationState` "NewEnumerator6"))
  (if (`local.isDeadLocal`)
    (set `local.AnimationState` "NewEnumerator5"))
  (return (select `/Game/Data/AnimationState` (`local.AnimationState`) :`NewEnumerator0` (`self.IdleFlipbook`) :`NewEnumerator1` (`self.RunFlipbook`) :`NewEnumerator2` (`self.JumpingFlipbook`) :`NewEnumerator3` (`self.FallingFlipbook`) :`NewEnumerator4` (`self.DoubleJumpingFlipbook`) :`NewEnumerator5` (`self.DeadFlipbook`) :`NewEnumerator6` (`self.ShootingFlipbook`))))

(fn `Shoot`
  (`|SpawnActorFromClass` "/Game/Blueprints/CharacterProjectile.CharacterProjectile_C" (`KismetMathLibrary.MakeTransform` (+ (`self.K2_GetActorLocation`) (0.0 -10.0 0.0)) (`KismetMathLibrary.ComposeRotators` (struct :`Pitch` -90.0) (`self.K2_GetActorRotation`))) "Undefined" "OverrideRootScale" null null))

(fn `UserConstructionScript`)