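; Player projectile actor that awards points for dead enemies and bosses and cleans itself up.
; On overlap it ignores MainCharacter, adds the Value of an already-dead Enemy or Boss to its owning MainCharacter's Points, then destroys itself without applying damage.
; A hit destroys it immediately against an EnemyProjectile, or after a short delay otherwise.
; A lifespan set on BeginPlay removes stray shots.
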(event `self.ReceiveBeginPlay`
  (`self.SetLifeSpan` 6.0))

(event `self.ReceiveActorBeginOverlap`
  (params (OtherActor :type "Actor Object Reference"))
  (cast `/Game/Blueprints/MainCharacter` OtherActor
    (:`CastFailed`
      (bind _asenemy (cast `/Game/Blueprints/Enemy` OtherActor)
        (:`then`
          (bind _asmain_character (cast `/Game/Blueprints/MainCharacter` (`self.GetOwner`))
            (:`then`
              (if (`/Game/Blueprints/Enemy.is Dead` _asenemy)
                (set `/Game/Blueprints/MainCharacter.Points` (+ (`/Game/Blueprints/MainCharacter.Points` _asmain_character) (`/Game/Blueprints/Enemy.Value` _asenemy)) _asmain_character)))
            (:`CastFailed`
              _)))
        (:`CastFailed`
          (bind _asboss (cast `/Game/Blueprints/Boss` OtherActor)
            (:`then`
              (bind _asmain_character_2 (cast `/Game/Blueprints/MainCharacter` (`self.GetOwner`))
                (:`then`
                  (if (`/Game/Blueprints/Boss.is Dead` _asboss)
                    (set `/Game/Blueprints/MainCharacter.Points` (+ (`/Game/Blueprints/MainCharacter.Points` _asmain_character_2) (`/Game/Blueprints/Boss.Value` _asboss)) _asmain_character_2)))
                (:`CastFailed`
                  _)))
            (:`CastFailed`
              _))))
      (`self.K2_DestroyActor` :!label _label))))

(event `self.ReceiveHit`
  (params (MyComp :type "PrimitiveComponent Object Reference") (Other :type "Actor Object Reference") (OtherComp :type "PrimitiveComponent Object Reference") (bSelfMoved :type Boolean) (HitLocation :type "Vector Structure") (HitNormal :type "Vector Structure") (NormalImpulse :type "Vector Structure") (Hit :type "HitResult Structure (by ref)"))
  (cast `/Game/Blueprints/EnemyProjectile` Other
    (:`then`
      (goto _label))
    (:`CastFailed`
      (`KismetSystemLibrary.Delay` 0.2)
      (goto _label))))

(fn `UserConstructionScript`
  (locals (Damage :type Integer :default 2)))